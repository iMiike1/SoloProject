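; Game state for the lobby that runs the countdown before the lobby game mode triggers travel.
; A looping one-second timer started on BeginPlay decrements Time and splits it into RemainingMins and RemainingSeconds.
; At zero or below it calls Travel on LobbyGameMode; the timer is never cleared, so the call repeats each second while the state remains active.
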(event `self.ReceiveBeginPlay`
  (`KismetSystemLibrary.K2_SetTimer` null "GameTimer" 1.0 true))

(fn `GameTimer`
  (bind _time (`self.Time`))
  (`/Engine/EditorBlueprintResources/StandardMacros.DecrementInt` (`self.Time`)
    (:`  `
      (set `self.RemainingMins` (/ _time 60))
      (set `self.RemainingSeconds` (mod _time 60))
      (if (<= (`self.Time`) 0)
        (bind _aslobby_game_mode (cast `/Game/Blueprints/LobbyGameMode` (`GameplayStatics.GetGameMode`)))
        (`/Game/Blueprints/LobbyGameMode.Travel` _aslobby_game_mode)))))

(fn `UserConstructionScript`)